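; Walking enemy that patrols a list of points back and forth, reacts to noise, and chases and attacks the player.
; PawnSensing drives it: noise sets a look rotation applied on Tick, while seeing a Player-tagged pawn locks the target and starts an AI MoveTo chase.
; Reaching the target starts a looping damage timer, which Tick stops beyond melee range, dropping the target outside sight radius.
; Taking damage triggers a brief crouch.
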(event OnHearNoise(PawnSensing)
  (params (Instigator :type Pawn%20Object%20Reference) (Location :type Vector%20%28by%20ref%29 :default "0, 0, 0") (Volume :type Float%20%28single-precision%29))
  (if (not (Variables|Default|GetDistracted))
    (Variables|Default|SetDistracted true)
    (Variables|Default|SetShouldLook true)
    (Variables|Default|SetTargetLookRotaton (Math|Rotator|FindLookatRotation (Transformation|GetWorldLocation (Variables|Default|GetCapsuleComponent)) Location))
    (Utilities|FlowControl|Delay (Variables|Default|GetAlarmTime))
    (if (not (Variables|Default|GetDistracted))
      (CallFunction|BacktoNormal))))

(event OnSeePawn(PawnSensing)
  (params (Pawn :type Pawn%20Object%20Reference))
  (if (Actor|ActorHasTag Pawn "Player")
    (Variables|Default|SetShouldLook false)
    (Variables|Default|SetDistracted true)
    (Variables|Default|SetLockedTarget Pawn)
    (CallFunction|StartChasing)))

(event Custom|Attack
  (Game|Damage|ApplyDamage (Variables|Default|GetLockedTarget) (Variables|Default|GetDamage) 0 0))

(event Custom|StopAttack
  (bind _attack_timer (Variables|Default|GetAttack_Timer))
  (Utilities|FlowControl|Delay (Utilities|Time|GetTimerRemainingTimebyHandle _attack_timer))
  (Utilities|Time|ClearandInvalidateTimerbyHandle _attack_timer))

(event Custom|StartChasing
  (AI|AIMoveTo self "0, 0, 0" (Variables|Default|GetLockedTarget) 1.5e+02 false
    (:OnSuccess
      (if (not (Utilities|Time|IsValidTimerHandle (Variables|Default|GetAttack_Timer)))
        (bind _returnvalue (Utilities|Time|SetTimerbyEvent (delegate Custom|Attack) (Variables|Default|GetAttackInterval) true))
        (Variables|Default|SetAttack_Timer _returnvalue)
        (CallFunction|Attack)))))

(event Custom|GoToPoint
  (bind _points (Variables|Default|GetPoints))
  (bind _returnvalue (Utilities|Array|Length _points))
  (if (> _returnvalue 0)
    (AI|AIMoveTo self "0, 0, 0" (Utilities|Array|Get(acopy) _points (Variables|Default|GetCurrentPoint)) 1e+02 false
      (:OnSuccess
        (if (Math|Integer|InRange(Integer) (+ (Variables|Default|GetCurrentPoint) (Variables|Default|GetDirection)) 0 _returnvalue true false)
          _
          (else
            (Variables|Default|SetDirection (* (Variables|Default|GetDirection) -1))))
        (Variables|Default|SetCurrentPoint (+ (Variables|Default|GetCurrentPoint) (Variables|Default|GetDirection)))
        (if (> _returnvalue 1)
          (CallFunction|GotoPoint))))))

(event EventBeginPlay
  (|CallParentFunction)
  (Variables|Default|SetDefaultLocation (Transformation|GetActorLocation))
  (CallFunction|GotoPoint))

(event EventTick
  (params (DeltaSeconds :type Float%20%28single-precision%29))
  (Utilities|IsValid (Variables|Default|GetLockedTarget)
    (:Is%20Valid
      (if (> (Transformation|GetDistanceTo (Variables|Default|GetLockedTarget) self) 2e+02)
        (CallFunction|StopAttack)
        (if (>= (Transformation|GetDistanceTo (Variables|Default|GetLockedTarget) self) (Variables|/Script/AIModule.PawnSensingComponent|GetSightRadius (Variables|Default|GetPawnSensing)))
          (Components|Movement|StopMovementImmediately (Variables|Character|GetCharacterMovement))
          (Variables|Default|SetLockedTarget 0)
          (if (Variables|Default|GetShouldLook) :!label _label
            (CallFunction|LookatLocation)))))
    (:Is%20Not%20Valid
      (goto _label))))

(event Game|Damage|EventAnyDamage
  (params (Damage :type Float%20%28single-precision%29) (DamageType :type Damage%20Type%20Object%20Reference) (InstigatedBy :type Controller%20Object%20Reference) (DamageCauser :type Actor%20Object%20Reference))
  (if (not (AI|Components|NavMovement|IsCrouching (Variables|Character|GetCharacterMovement)))
    (Character|Crouch)
    (Utilities|FlowControl|Delay 1.5)
    (Character|UnCrouch)))

(fn ConstructionScript
  (|CallParentFunction))