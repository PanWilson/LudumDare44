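; Stationary-style enemy that turns toward players it sees and fires projectiles at them on a looping timer.
; PawnSensing sight locks a player target until it leaves sight radius, while heard noises briefly turn the enemy toward the sound.
; Tick smoothly interpolates capsule yaw toward the look rotation, returning to the starting rotation after an alarm delay.
; Shots get slight random yaw spread, and taking damage briefly pauses the attack timer.
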(event OnHearNoise(PawnSensing)
  (params (Instigator :type Pawn%20Object%20Reference) (Location :type Vector%20%28by%20ref%29 :default "0, 0, 0") (Volume :type Float%20%28single-precision%29))
  (if (not (Variables|Default|GetDistracted))
    (Variables|Default|SetDistracted true)
    (Variables|Default|SetShouldLook true)
    (Variables|Default|SetTargetLookRotaton (Math|Rotator|FindLookatRotation (Transformation|GetWorldLocation (Variables|Collision|GetCapsuleComponent)) Location))
    (Utilities|FlowControl|Delay (Variables|Default|GetAlarmTime))
    (CallFunction|BacktoNormal)))

(event OnSeePawn(PawnSensing)
  (params (Pawn :type Pawn%20Object%20Reference))
  (if (and (Pawn|IsPlayerControlled Pawn) (not (Utilities|IsValid (Variables|Default|GetLockedTarget))))
    (Variables|Default|SetLockedTarget Pawn)
    (bind _returnvalue (Utilities|Time|SetTimerbyEvent (delegate Custom|Shoot) (Variables|Default|GetAttackInterval) true))
    (Variables|Default|SetAttack_Timer _returnvalue)))

(event Custom|Shoot
  (bind _capsulecomponent (Variables|Collision|GetCapsuleComponent))
  (bind _returnvalue (Transformation|GetWorldRotation _capsulecomponent))
  (bind (_roll _pitch _yaw) (Math|Rotator|BreakRotator _returnvalue))
  (Game|SpawnActorfromClass "/Game/Blueprints/Enemy/BaseProjectile.BaseProjectile_C" (Math|Transform|MakeTransform (Transformation|GetWorldLocation _capsulecomponent) (Math|Rotator|MakeRotator _roll _pitch (+ _yaw (Math|Random|RandomFloatinRange -3.0 3.0)))) "Undefined" 0 self))

(event Custom|LookAtLocation
  (bind _capsulecomponent (Variables|Collision|GetCapsuleComponent))
  (bind _targetlookrotaton (Variables|Default|GetTargetLookRotaton))
  (bind _yaw (Math|Rotator|BreakRotator _targetlookrotaton))
  (bind _returnvalue (Transformation|GetWorldRotation _capsulecomponent))
  (bind (_roll _pitch) (Math|Rotator|BreakRotator _returnvalue))
  (bind _returnvalue_2 (Math|Rotator|MakeRotator _roll _pitch _yaw))
  (if (Utilities|Enum|NotEqual(Enum) _returnvalue _returnvalue_2)
    (Transformation|SetWorldRotation (Variables|Collision|GetCapsuleComponent) (Math|Interpolation|RInterpTo _returnvalue _returnvalue_2 (Utilities|Time|GetWorldDeltaSeconds) (Variables|Default|GetRotateSpeed)) false false)
    (else
      (Variables|Default|SetShouldLook false))))

(event Custom|BackToNormal
  (Variables|Default|SetDistracted false)
  (Variables|Default|SetShouldLook true)
  (Variables|Default|SetTargetLookRotaton (Variables|Default|GetDefaultRotation)))

(event EventBeginPlay
  (Variables|Default|SetDefaultRotation (Transformation|GetWorldRotation (Variables|Collision|GetCapsuleComponent))))

(event EventTick
  (params (DeltaSeconds :type Float%20%28single-precision%29))
  (Utilities|IsValid (Variables|Default|GetLockedTarget)
    (:Is%20Valid
      (if (<= (Transformation|GetDistanceTo (Variables|Default|GetLockedTarget) self) (Variables|/Script/AIModule.PawnSensingComponent|GetSightRadius (Variables|Default|GetPawnSensing)))
        (Variables|Default|SetTargetLookRotaton (Math|Rotator|FindLookatRotation (Transformation|GetWorldLocation (Variables|Collision|GetCapsuleComponent)) (Transformation|GetActorLocation (Variables|Default|GetLockedTarget))))
        (Variables|Default|SetDistracted true)
        (CallFunction|LookatLocation :!label _label)
        (else
          (Variables|Default|SetLockedTarget 0)
          (Utilities|Time|ClearandInvalidateTimerbyHandle (Variables|Default|GetAttack_Timer))
          (Utilities|FlowControl|Delay (Variables|Default|GetAlarmTime))
          (CallFunction|BacktoNormal)
          (if (Variables|Default|GetShouldLook) :!label _label_2
            (goto _label)))))
    (:Is%20Not%20Valid
      (goto _label_2))))

(event Game|Damage|EventAnyDamage
  (params (Damage :type Float%20%28single-precision%29) (DamageType :type Damage%20Type%20Object%20Reference) (InstigatedBy :type Controller%20Object%20Reference) (DamageCauser :type Actor%20Object%20Reference))
  (bind _attack_timer (Variables|Default|GetAttack_Timer))
  (if (Utilities|Time|IsValidTimerHandle _attack_timer)
    (Utilities|Time|PauseTimerbyHandle _attack_timer)
    (Utilities|FlowControl|Delay 1.5)
    (Utilities|Time|UnpauseTimerbyHandle _attack_timer)))

(fn ConstructionScript)