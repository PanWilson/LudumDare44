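; Pile is a storage Blueprint that tracks a bounded capacity and flags whether it can accept input or give output.
; BeginPlay sets CanInput and CanOutput from the starting amount.
; ChangeCapacity adds a value clamped between zero and MaxCapacity, updates a text render with the total, and refreshes both flags.
; Its Full and Empty events switch off input and output respectively at the limits.
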(event Custom|ChangeCapacity
  (params (Value :type Float%20%28single-precision%29))
  (bind _output_get (Variables|Default|SetCurrentCapacity (Math|Float|Clamp(Float) (+ Value (Variables|Default|GetCurrentCapacity)) 0.0 (Variables|Default|GetMaxCapacity))))
  (Rendering|Components|TextRender|SetText (Variables|Default|GetTextRender) (Utilities|Text|ToText(Float) _output_get "HalfToEven"))
  (if (<= _output_get 0.0)
    (CallFunction|Empty)
    (else
      (Variables|Default|SetCanOutput true)))
  (if (>= _output_get (Variables|Default|GetMaxCapacity))
    (CallFunction|Full)
    (else
      (Variables|Default|SetCanInput true))))

(event Custom|Full
  (Variables|Default|SetCanInput false))

(event Custom|Empty
  (Variables|Default|SetCanOutput false))

(event EventBeginPlay
  (if (== (Variables|Default|GetCurrentCapacity) 0.0)
    (Variables|Default|SetCanInput true)
    (Variables|Default|SetCanOutput false)
    (elif (== (Variables|Default|GetCurrentCapacity) (Variables|Default|GetMaxCapacity))
      (Variables|Default|SetCanInput false)
      (Variables|Default|SetCanOutput true)
      (else
        (Variables|Default|SetCanInput true)
        (Variables|Default|SetCanOutput true)))))

(fn ConstructionScript)