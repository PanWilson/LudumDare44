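; CoinProjectile is a bouncing coin projectile that makes noise and can damage enemies.
; Each bounce reports noise at the sphere's location, attributed to the instigator, and draws a brief red debug point there.
; Sphere hits apply the Damage variable to actors carrying the "Enemy" tag.
; The coin destroys itself when its projectile movement stops.
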(event OnProjectileStop(ProjectileMovement)
  (params (ImpactResult :type Hit%20Result%20Structure%20%28by%20ref%29))
  (Actor|DestroyActor))

(event OnProjectileBounce(ProjectileMovement)
  (params (ImpactResult :type Hit%20Result%20Structure%20%28by%20ref%29) (ImpactVelocity :type Vector%20%28by%20ref%29 :default "0, 0, 0"))
  (bind _sphere (Variables|Default|GetSphere))
  (bind _returnvalue (Transformation|GetWorldLocation _sphere))
  (Class|Actor|MakeNoise 1.0 (Variables|Actor|GetInstigator) _returnvalue 1.0 "None")
  (Rendering|Debug|DrawDebugPoint _returnvalue 5.0 "(R=1.000000,G=0.000000,B=0.000000,A=1.000000)" 2.0))

(event OnComponentHit(Sphere)
  (params (HitComponent :type Primitive%20Component%20Object%20Reference) (OtherActor :type Actor%20Object%20Reference) (OtherComp :type Primitive%20Component%20Object%20Reference) (NormalImpulse :type Vector :default "0, 0, 0") (Hit :type Hit%20Result%20Structure%20%28by%20ref%29))
  (for _array_element (Variables|/Script/Engine.Actor|GetTags OtherActor)
    (if (Utilities|Name|Equal(Name) _array_element "Enemy")
      (Game|Damage|ApplyDamage OtherActor (Variables|Default|GetDamage) 0 0))))

(event EventBeginPlay)

(event Collision|EventActorBeginOverlap
  (params (OtherActor :type Actor%20Object%20Reference)))

(event EventTick
  (params (DeltaSeconds :type Float%20%28single-precision%29)))

(fn ConstructionScript)