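; Player character whose coin count drives bag scale and text, pays for shots, drops with damage, and disables input at zero.
; Holding Interact on a tagged Pile under the cursor runs looping timers that move coins in or out; stopping hands the fractional remainder to the pile.
; The capsule turns toward the cursor every tick and moves by speed-limited forces.
; Shoot spawns a gravity-free coin projectile along its facing.
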(event Custom|RotateTowardsCursor
  (bind _returnvalue (Game|GetPlayerController 0))
  (bind _capsule (Variables|Default|GetCapsule))
  (bind (_hitresult _returnvalue_2) (Game|Player|GetHitResultUnderCursorbyChannel _returnvalue "TraceTypeQuery2" false))
  (bind _returnvalue_3 (Transformation|GetWorldRotation _capsule))
  (bind (_roll _pitch) (Math|Rotator|BreakRotator _returnvalue_3))
  ;[1 1 1] Movement
  (if _returnvalue_2
    (Transformation|SetWorldRotation _capsule (Math|Rotator|MakeRotator _roll _pitch (.Yaw (Math|Rotator|BreakRotator (Math|Rotator|FindLookatRotation (Transformation|GetWorldLocation (Variables|Default|GetCapsule)) (.Location (Collision|BreakHitResult _hitresult)))))) false false)))

(event Custom|UpdateBag
  (Transformation|SetWorldScale3D (Variables|Default|GetBag) (Math|Conversions|ToVector(Float) (Math|Float|Clamp(Float) (/ (Variables|Bag|GetCurrentCapacity) (Variables|Bag|GetBaseCapacity)) 0.1 1e+02))))

(event Custom|StopCoinInput
  (bind _coininputtimer (Variables|Bag|GetCoinInputTimer))
  ;[1 1 1] CoinInput
  (if (Utilities|Time|IsValidTimerHandle _coininputtimer)
    (Utilities|Time|ClearandInvalidateTimerbyHandle _coininputtimer)
    (bind _roundeddifference (CallFunction|RoundCapacity))
    (Default|ChangeCapacity (Variables|Bag|GetTransactionTarget) _roundeddifference)
    (Variables|Bag|SetTransactionTarget 0)))

(event Custom|ChangeCoinAmount
  (params (Value :type Float%20%28single-precision%29))
  (bind _output_get (Variables|Bag|SetCurrentCapacity (Math|Float|Clamp(Float) (+ (Variables|Bag|GetCurrentCapacity) Value) 0.0 (Variables|Bag|GetMaxCapacity))))
  (CallFunction|UpdateBag)
  (Rendering|Components|TextRender|SetText (Variables|Default|GetTextRender) (Utilities|Text|ToText(Float) _output_get "HalfToEven"))
  (if (>= _output_get (Variables|Bag|GetMaxCapacity))
    (CallFunction|Full)
    (else
      (Variables|Bag|SetCanInput true)))
  (if (<= _output_get 0.0)
    (CallFunction|Empty)
    (else
      (Variables|Bag|SetCanOutput true))))

(event Custom|StartCoinOutput
  ;[1 1 1] Coin Output
  (bind _returnvalue (Utilities|Time|SetTimerbyEvent (delegate Custom|CoinOutput) 0.1 true))
  (Variables|Bag|SetCoinOutputTimer _returnvalue)
  (CallFunction|CoinOutput))

(event Custom|CoinOutput
  (bind _outputspeed (Variables|Bag|GetOutputSpeed))
  (bind _transactiontarget (Variables|Bag|GetTransactionTarget))
  (bind _returnvalue (/ _outputspeed 1e+01))
  ;[1 1 1] Coin Output
  (if (and (Variables|/Game/Blueprints/Pile.Pile_C|GetCanInput _transactiontarget) (Variables|Bag|GetCanOutput))
    (CallFunction|ChangeCoinAmount (* _returnvalue -1.0))
    (Utilities|IsValid _transactiontarget
      (:Is%20Valid
        (Default|ChangeCapacity _transactiontarget _returnvalue))
      (:Is%20Not%20Valid
        (CallFunction|StopCoinOutput :!label _label)))
    (else
      (goto _label))))

(event Custom|Full
  (Variables|Bag|SetCanInput false))

(event Custom|Empty
  (Variables|Bag|SetCanOutput false)
  (Input|DisableInput 0))

(event Custom|StopCoinOutput
  (bind _coinoutputtimer (Variables|Bag|GetCoinOutputTimer))
  ;[1 1 1] Coin Output
  (if (Utilities|Time|IsValidTimerHandle _coinoutputtimer)
    (Utilities|Time|ClearandInvalidateTimerbyHandle _coinoutputtimer)
    (bind _roundeddifference (CallFunction|RoundCapacity))
    (Default|ChangeCapacity (Variables|Bag|GetTransactionTarget) _roundeddifference)
    (Variables|Bag|SetTransactionTarget 0)))

(event Custom|StartCoinInput
  ;[1 1 1] CoinInput
  (bind _returnvalue (Utilities|Time|SetTimerbyEvent (delegate Custom|CoinInput) 0.1 true))
  (Variables|Bag|SetCoinInputTimer _returnvalue)
  (CallFunction|CoinInput))

(event Custom|CoinInput
  (bind _transactiontarget (Variables|Bag|GetTransactionTarget))
  (bind _inputspeed (Variables|Bag|GetInputSpeed))
  (bind _returnvalue (/ _inputspeed 1e+01))
  ;[1 1 1] CoinInput
  (if (and (Variables|/Game/Blueprints/Pile.Pile_C|GetCanOutput _transactiontarget) (Variables|Bag|GetCanInput))
    (CallFunction|ChangeCoinAmount _returnvalue)
    (Utilities|IsValid _transactiontarget
      (:Is%20Valid
        (Default|ChangeCapacity _transactiontarget (* _returnvalue -1.0)))
      (:Is%20Not%20Valid
        (CallFunction|StopCoinInput :!label _label)))
    (else
      (goto _label))))

(event EventBeginPlay
  (Variables|Bag|SetCurrentCapacity (Variables|Bag|GetBaseCapacity)))

(event EventTick
  (params (DeltaSeconds :type Float%20%28single-precision%29))
  (CallFunction|RotateTowardsCursor))

(event Game|Damage|EventAnyDamage
  (params (Damage :type Float%20%28single-precision%29) (DamageType :type Damage%20Type%20Object%20Reference) (InstigatedBy :type Controller%20Object%20Reference) (DamageCauser :type Actor%20Object%20Reference))
  (CallFunction|ChangeCoinAmount (* Damage -1.0)))

(event Input|ActionEvents|InputActionInteract
  (params (Key :type Key%20Structure))
  (bind _returnvalue (Game|GetPlayerController 0))
  (bind (_hitresult _returnvalue_2) (Game|Player|GetHitResultUnderCursorbyChannel _returnvalue "TraceTypeQuery1" false))
  (bind _hitactor (Collision|BreakHitResult _hitresult))
  (:Pressed
    (if _returnvalue_2
      (bind _array_element (Utilities|Array|ForEachLoopwithBreak (Variables|/Script/Engine.Actor|GetTags _hitactor))
        (:LoopBody
          (switch name _array_element
            (:OPile
              (bind _aspile (Utilities|Casting|CastToPile _hitactor))
              (Variables|Bag|SetTransactionTarget _aspile)
              (CallFunction|StartCoinOutput))
            (:IPile
              (bind _aspile_2 (Utilities|Casting|CastToPile _hitactor))
              (Variables|Bag|SetTransactionTarget _aspile_2)
              (CallFunction|StartCoinInput)))))))
  (:Released
    (CallFunction|StopCoinOutput)
    (CallFunction|StopCoinInput)))

(event Input|ActionEvents|InputActionShoot
  (params (Key :type Key%20Structure))
  (bind _capsule (Variables|Default|GetCapsule))
  (:Pressed
    (CallFunction|ChangeCoinAmount (* (Variables|Throwing/Shooting|GetShootCost) -1.0))
    (bind _returnvalue (Game|SpawnActorfromClass "/Game/Blueprints/Character/CoinProjectile.CoinProjectile_C" (Math|Transform|MakeTransform (Transformation|GetWorldLocation _capsule) (Transformation|GetWorldRotation _capsule)) "Undefined" 0 self))
    (Variables|/Script/Engine.MovementComponent|SetVelocity (Variables|/Game/Blueprints/Character/CoinProjectile.CoinProjectile_C|GetProjectileMovement _returnvalue) (* (Math|Vector|GetForwardVector (Variables|Default|GetCapsule)) (Variables|Throwing/Shooting|GetShootSpeed)))
    (Variables|/Script/Engine.ProjectileMovementComponent|SetProjectileGravityScale (Variables|/Game/Blueprints/Character/CoinProjectile.CoinProjectile_C|GetProjectileMovement _returnvalue) 0.0)))

(event Input|ActionEvents|InputActionThrow
  (params (Key :type Key%20Structure)))

(event Input|AxisEvents|InputAxisMoveHorizontally
  (params (AxisValue :type Float%20%28single-precision%29))
  (bind _capsule (Variables|Default|GetCapsule))
  ;[1 1 1] Movement
  (if (<= (Math|Vector|VectorLength (Math|Vector|ProjectVectorontoPlane (Transformation|GetComponentVelocity _capsule) (Math|Vector|GetUpVector _capsule))) (Variables|Movement|GetMaxSpeed))
    (Physics|AddForce _capsule (* (Math|Vector|MakeVector (stale Input|AxisEvents|InputAxisMoveVertically AxisValue) AxisValue 0.0) (Variables|Movement|GetAcceleration)) "None" true)))

(event Input|AxisEvents|InputAxisMoveVertically
  (params (AxisValue :type Float%20%28single-precision%29))
  (bind _capsule (Variables|Default|GetCapsule))
  ;[1 1 1] Movement
  (if (<= (Math|Vector|VectorLength (Math|Vector|ProjectVectorontoPlane (Transformation|GetComponentVelocity _capsule) (Math|Vector|GetUpVector _capsule))) (Variables|Movement|GetMaxSpeed))
    (Physics|AddForce _capsule (* (Math|Vector|MakeVector AxisValue (stale Input|AxisEvents|InputAxisMoveHorizontally AxisValue) 0.0) (Variables|Movement|GetAcceleration)) "None" true)))

(fn ConstructionScript)

(fn RoundCapacity
  (bind _output_get (LocalVariables|Setcached (Math|Float|%(Float) (Variables|Bag|GetCurrentCapacity) 1.0)))
  (CallFunction|ChangeCoinAmount (* _output_get -1.0))
  (return _output_get))